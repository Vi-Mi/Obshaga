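; Level-transition trigger actor that saves progress and loads a named level when the player's BP_FPS_Character overlaps its box.
; SaveGame loads or creates a BP_SaveGame slot, then writes the target level, held and equipped item state, and the directional light's rotation as the sun.
; The overlap then plays a camera shutter sound, shows a Fade widget animation, and opens the level after a short delay.
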(event OnComponentBeginOverlap(Box)
  (params (OverlappedComponent :type Primitive%20Component%20Object%20Reference) (OtherActor :type Actor%20Object%20Reference) (OtherComp :type Primitive%20Component%20Object%20Reference) (OtherBodyIndex :type Integer) (bFromSweep :type Boolean) (SweepResult :type Hit%20Result%20Structure%20%28by%20ref%29))
  (Utilities|Casting|CastToBP_FPS_Character OtherActor)
  (CallFunction|SaveGame)
  (Audio|PlaySound2D "/Engine/VREditor/Sounds/UI/Camera_Shutter.Camera_Shutter" 1.0 1.0 0.0 0 0)
  (bind _returnvalue (UserInterface|CreateWidget "/Game/UI/Fade.Fade_C"))
  (UserInterface|Viewport|AddtoViewport _returnvalue 0)
  (Default|FadeAnimation _returnvalue)
  (Utilities|FlowControl|Delay 0.5)
  (Game|OpenLevel(byName) (Variables|Default|GetLevel%20Name)))

(event EventBeginPlay)

(event Collision|EventActorBeginOverlap
  (params (OtherActor :type Actor%20Object%20Reference)))

(event EventTick
  (params (DeltaSeconds :type Float%20%28single-precision%29)))

(fn ConstructionScript)

(fn SaveGame
  (bind _returnvalue (SaveGame|DoesSaveGameExist (Variables|Default|GetSaveName)))
  (if _returnvalue
    (bind _returnvalue_2 (SaveGame|LoadGamefromSlot (Variables|Default|GetSaveName)))
    (Variables|Default|SetSave%20REF _returnvalue_2)
    (else
      (bind _returnvalue_3 (SaveGame|CreateSaveGameObject "/Game/Blueprints/BP_SaveGame.BP_SaveGame_C"))
      (Variables|Default|SetSave%20REF _returnvalue_3)))
  (bind _asbp_save_game (Utilities|Casting|CastToBP_SaveGame (Variables|Default|GetSave%20REF)))
  (Variables|Default|SetSave _asbp_save_game)
  (Variables|/Game/Blueprints/BP_SaveGame.BP_SaveGame_C|SetLevel _asbp_save_game (Variables|Default|GetLevel%20Name))
  (bind _asbp_fps_character (Utilities|Casting|CastToBP_FPS_Character (Game|Player|GetPlayerPawn 0)))
  (Variables|/Game/Blueprints/BP_SaveGame.BP_SaveGame_C|SetInHand _asbp_save_game (Variables|/Game/Blueprints/Character/BP_FPS_Character.BP_FPS_Character_C|GetISIC_STATIC_MESH _asbp_fps_character))
  (Variables|/Game/Blueprints/BP_SaveGame.BP_SaveGame_C|SetHeldItemType _asbp_save_game (Variables|/Game/Blueprints/Character/BP_FPS_Character.BP_FPS_Character_C|GetHeldItemType _asbp_fps_character))
  (Variables|/Game/Blueprints/BP_SaveGame.BP_SaveGame_C|SetEquipedItemSave _asbp_save_game (Variables|/Game/Blueprints/Character/BP_FPS_Character.BP_FPS_Character_C|GetEquipedItem _asbp_fps_character))
  (Variables|/Game/Blueprints/BP_SaveGame.BP_SaveGame_C|SetEquipedItemStaticMesh _asbp_save_game (Variables|/Script/Engine.StaticMeshComponent|GetStaticMesh (Variables|/Game/Blueprints/Character/BP_FPS_Character.BP_FPS_Character_C|GetEquipedItem _asbp_fps_character)))
  (bind _returnvalue_4 (Actor|GetActorOfClass "/Script/Engine.DirectionalLight"))
  (Variables|/Game/Blueprints/BP_SaveGame.BP_SaveGame_C|SetSun _asbp_save_game (Transformation|GetActorRotation _returnvalue_4))
  (SaveGame|SaveGametoSlot (Variables|Default|GetSave) (Variables|Default|GetSaveName)))
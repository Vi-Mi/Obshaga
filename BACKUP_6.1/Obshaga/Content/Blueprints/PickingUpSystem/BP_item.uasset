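; BP_item is an item actor for the picking-up system that can be picked up and placed, with its mesh set from ItemModelToPlace at construction.
; PickUp disables physics on the mesh, prints a message, plays a sound and destroys the actor after a brief delay.
; Place prints a message and plays the Expand timeline.
; Tick clears the mesh's overlay material every frame, and an unused Shrink scale timeline remains, noted as broken with physics.
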(event EventBeginPlay)

(event EventTick
  (params (DeltaSeconds :type Float%20%28single-precision%29))
  (Rendering|Material|SetOverlayMaterial (Variables|Default|GetItemModel) 0 :!class /Script/Engine.MeshComponent))

(event EventPickUp
  (Physics|SetSimulatePhysics (Variables|Default|GetItemModel) false)
  (Development|PrintString "Item picked")
  (Audio|PlaySound2D "/Engine/VREditor/Sounds/UI/Object_PickUp.Object_PickUp" 1.0 1.0 0.0 0 0)
  ;[1 0.645 0.645] change delsy to 0.4, if there an animation
  (Utilities|FlowControl|Delay 0.05)
  (Actor|DestroyActor))

(event EventPlace
  (Development|PrintString "Item placed")
  (Timeline|Expand Play))

(fn ConstructionScript
  (Components|StaticMesh|SetStaticMesh (Variables|Default|GetItemModel) (Variables|Default|GetItemModelToPlace)))
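; Player stats component for the FPS character, holding health, speed factor, damage and the list of active power-ups.
; Health changes update the HUD bar and text; damage also plays a random hurt sound behind a two-second cooldown and reports death.
; Speed and damage reset to defaults on BeginPlay.
; Power-ups can be added from a type-to-info map, with remaining times updated or removed by index.
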(event Custom|SetOuchAndDisableItAfter
  (Variables|Damage|SetouchIsPlaying true)
  (Utilities|FlowControl|Delay 2.0)
  (Variables|Damage|SetouchIsPlaying false))

(event EventBeginPlay
  (Utilities|FlowControl|Sequence
    (:then_0
      (bind _asbp_fps_character (Utilities|Casting|CastToBP_FPS_Character (Components|GetOwner)))
      (Variables|Default|SetPlayer%20Character%20BP _asbp_fps_character))
    (:then_1
      (Speed|ResetSpeedFactor))
    (:then_2
      (Damage|ResetCurrentDamage))))

(fn DecreaseHealth
  (params (Damage :type Float%20%28double-precision%29))
  (bind _player_character_bp (Variables|Default|GetPlayer%20Character%20BP))
  (bind _hud_widget (Variables|/Game/Blueprints/Character/BP_FPS_Character.BP_FPS_Character_C|GetHUD%20Widget _player_character_bp))
  (bind _output_get (Variables|Health|SetCurrent%20Health (- (Variables|Health|GetCurrent%20Health) Damage)))
  (Progress|SetPercent (Variables|/Game/UI/BP_UI.BP_UI_C|GetHealthBar _hud_widget) (/ _output_get (Variables|Health|GetMax%20Health)))
  (Rendering|Components|TextRender|SetText (Variables|/Game/UI/BP_UI.BP_UI_C|GetHealthText _hud_widget) (Utilities|Text|ToText(Float) (Variables|Health|GetCurrent%20Health) "HalfToEven"))
  (Damage|PlayRandomSoundOuch)
  (if (<= (Variables|Health|GetCurrent%20Health) 0.0)
    (return true)
    (else
      (return false))))

(fn IncreaseMaxHealth
  (params (Health%20Incremention :type Float%20%28double-precision%29))
  (bind _player_character_bp (Variables|Default|GetPlayer%20Character%20BP))
  (bind _hud_widget (Variables|/Game/Blueprints/Character/BP_FPS_Character.BP_FPS_Character_C|GetHUD%20Widget _player_character_bp))
  (Variables|Health|SetMax%20Health (+ (Variables|Health|GetMax%20Health) Health%20Incremention))
  (Progress|SetPercent (Variables|/Game/UI/BP_UI.BP_UI_C|GetHealthBar _hud_widget) (/ (Variables|Health|GetCurrent%20Health) (Variables|Health|GetMax%20Health)))
  (Rendering|Components|TextRender|SetText (Variables|/Game/UI/BP_UI.BP_UI_C|GetHealthText _hud_widget) (Utilities|Text|ToText(Float) (Variables|Health|GetCurrent%20Health) "HalfToEven")))

(fn IncreaseHealth
  (params (Added%20Health :type Float%20%28double-precision%29))
  (bind _player_character_bp (Variables|Default|GetPlayer%20Character%20BP))
  (bind _hud_widget (Variables|/Game/Blueprints/Character/BP_FPS_Character.BP_FPS_Character_C|GetHUD%20Widget _player_character_bp))
  (Variables|Health|SetCurrent%20Health (+ (Variables|Health|GetCurrent%20Health) Added%20Health))
  (if (> (Variables|Health|GetCurrent%20Health) (Variables|Health|GetMax%20Health))
    (Variables|Health|SetCurrent%20Health (Variables|Health|GetMax%20Health)))
  (Progress|SetPercent (Variables|/Game/UI/BP_UI.BP_UI_C|GetHealthBar _hud_widget) (/ (Variables|Health|GetCurrent%20Health) (Variables|Health|GetMax%20Health)))
  (Rendering|Components|TextRender|SetText (Variables|/Game/UI/BP_UI.BP_UI_C|GetHealthText _hud_widget) (Utilities|Text|ToText(Float) (Variables|Health|GetCurrent%20Health) "HalfToEven")))

(fn PlayRandomSoundOuch
  (if (not (Variables|Damage|GetouchIsPlaying))
    (CallFunction|SetOuchandDisableItAfter)
    (if (Math|Random|RandomBool)
      (if (Math|Random|RandomBool)
        (Audio|PlaySound2D "/Game/Audio/fromInternet/classic_hurt.classic_hurt" 1.0 1.0 0.0 0 0)
        (else
          (Audio|PlaySound2D "/Game/Audio/fromInternet/oh_shit.oh_shit" 1.0 1.0 0.0 0 0)))
      (else
        (Audio|PlaySound2D "/Game/Audio/fromInternet/ouch.ouch" 1.0 1.0 0.0 0 0)))))

(fn SetSpeedFactor
  (params (New%20Speed%20Factor :type Float%20%28double-precision%29))
  (Variables|Speed|SetSpeed%20Factor New%20Speed%20Factor))

(fn GetSpeedFactor
  (return (Variables|Speed|GetSpeed%20Factor)))

(fn ResetSpeedFactor
  (Speed|SetSpeedFactor (Variables|Speed|GetDefault%20Speed%20Factor)))

(fn SetCurrentDamage
  (params (New%20Current%20Damage :type Float%20%28double-precision%29))
  (Variables|Damage|SetCurrent%20Damage New%20Current%20Damage))

(fn GetCurrentDamage
  (return (Variables|Damage|GetCurrent%20Damage)))

(fn ResetCurrentDamage
  (Damage|SetCurrentDamage (Variables|Damage|GetDefault%20Damage)))

(fn GetActivePowerUps
  (return (Variables|PowerUpsData|GetActivePowerUps)))

(fn AddActivePowerUp
  (params (NewParam :type Struct%20Power%20Up%20Info%20Structure))
  (Utilities|Array|Add (Variables|PowerUpsData|GetActivePowerUps) NewParam))

(fn SetActivePowerUp
  (params (Active%20Power%20Up :type Array%20of%20Struct%20Power%20Up%20Info%20Structures))
  (Variables|PowerUpsData|SetActivePowerUps Active%20Power%20Up))

(fn UpdateRemaingTimeatIndex
  (params (New%20Remaining%20Time :type Float%20%28double-precision%29) (Index :type Integer))
  (Utilities|Struct|SetmembersinStruct_PowerUpInfo (Utilities|Array|Get(acopy) (Variables|PowerUpsData|GetActivePowerUps) Index) New%20Remaining%20Time))

(fn DeleteRemainingTimeatIndex
  (params (Index :type Integer))
  (Utilities|Array|RemoveIndex (Variables|PowerUpsData|GetActivePowerUps) Index))

(fn AddActivePowerUpbyType
  (params (Power%20Up%20Type :type EPowerUpType%20Enum :default "NewEnumerator3"))
  (bind _powerupsmap (Variables|PowerUpsData|GetPowerUpsMap))
  (bind (_value _returnvalue) (Utilities|Map|Find _powerupsmap Power%20Up%20Type))
  (if _returnvalue
    (PowerUpsData|AddActivePowerUp _value)))
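; First-person player character with movement, a one-slot item pick up and place system, punching, pointing, HUD, and death that deletes the save and opens MainMenu.
; A shared camera line trace drives per-tick outline highlights, pickup, placement and terminal use.
; Holding the ISIC item turns terminal outlines green and lets E cycle tagged turnstiles open and closed.
; An enum step machine runs a key-by-key controls tutorial from BeginPlay, prompting via PrintString.
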(event Custom|PointHand
  ;[1 1 1] Point Hand Event
  (Audio|PlaySound2D "/Game/Audio/huh.huh" 1.0 1.0 0.0 0 0)
  (Variables|Turniket|SetIsPointingHand true)
  (Animation|PlayAnimMontage "/Game/Animations/PointingAnimation_Montage.PointingAnimation_Montage" 1.0 "None")
  (Utilities|FlowControl|Delay 1.5)
  (Variables|Turniket|SetIsPointingHand false))

(event Custom|Place%20Item
  ;[1 1 1] Place item
  (Rendering|SetVisibility (Variables|Default|GetEquipedItem) false false)
  (bind _outhit (CallFunction|GetRayTracedItem (Variables|PickUpSystem|GetPlaceDistance)))
  (Game|SpawnActorfromClass "/Game/Blueprints/PickingUpSystem/BP_item.BP_item_C" (Math|Transform|MakeTransform (CallFunction|TakeLocationforPlace (.Location (Collision|BreakHitResult _outhit)) (.TraceEnd (Collision|BreakHitResult _outhit))) "0, 0, 0" "1.000000,1.000000,1.000000") "Undefined" "MultiplyWithRoot" 0 (Variables|/Script/Engine.StaticMeshComponent|GetStaticMesh (Variables|Default|GetEquipedItem)) (Variables|Inventar|GetHeldItemType) 0)
  (Variables|Inventar|SetHeldItemType "NewEnumerator0")
  (Audio|PlaySound2D "/Game/Audio/place_item.place_item" 1.0 1.0 0.0 0 0))

(event Custom|Diying%20logic
  ;[1 1 1] Dying logic
  (CallFunction|Die)
  (Utilities|FlowControl|Delay 3.0)
  (Actor|DestroyActor)
  (Game|OpenLevel(byName) "MainMenu"))

(event Custom|Glowing%20Effect
  ;[1 1 1] Glowing effect on pickable item
  (bind (_outhit _returnvalue) (CallFunction|GetRayTracedItem (Variables|PickUpSystem|GetPickUpItemDistance)))
  (if _returnvalue
    (bind _asbp_item (Utilities|Casting|CastToBP_item (.HitActor (Collision|BreakHitResult _outhit)))
      (:then
        (Rendering|Material|SetOverlayMaterial (Variables|/Game/Blueprints/PickingUpSystem/BP_item.BP_item_C|GetItemModel _asbp_item) "/Game/Materials/M_Outline.M_Outline" :!class /Script/Engine.MeshComponent))
      (:CastFailed
        ;;[1 0.3564 0.3564] Termnal effect
        (bind _asbp_terminal (Utilities|Casting|CastToBP_Terminal (.HitActor (Collision|BreakHitResult _outhit))))
        (if (CallFunction|HasIsicFunc)
          (Rendering|Material|SetOverlayMaterial (Variables|/Script/Engine.StaticMeshActor|GetStaticMeshComponent _asbp_terminal) "/Game/Materials/M_OutlineG.M_OutlineG" :!class /Script/Engine.MeshComponent)
          (else
            (Rendering|Material|SetOverlayMaterial (Variables|/Script/Engine.StaticMeshActor|GetStaticMeshComponent _asbp_terminal) "/Game/Materials/M_OutlineR.M_OutlineR" :!class /Script/Engine.MeshComponent)))))))

(event Custom|Pick%20Up%20Item
  ;[1 1 1] Pick Up Item
  (bind (_outhit _returnvalue) (CallFunction|GetRayTracedItem (Variables|PickUpSystem|GetPickUpItemDistance)))
  (if _returnvalue
    (bind _asbp_item (Utilities|Casting|CastToBP_item (.HitActor (Collision|BreakHitResult _outhit))))
    (Class|BPIItems|PickUp(Message) _asbp_item)
    (Components|StaticMesh|SetStaticMesh (Variables|Default|GetEquipedItem) (Variables|/Script/Engine.StaticMeshComponent|GetStaticMesh (Variables|/Game/Blueprints/PickingUpSystem/BP_item.BP_item_C|GetItemModel _asbp_item)))
    (Rendering|SetVisibility (Variables|Default|GetEquipedItem) true false)
    (Variables|Inventar|SetHeldItemType (Variables|/Game/Blueprints/PickingUpSystem/BP_item.BP_item_C|GetItemType _asbp_item))))

(event EventBeginPlay
  ;[1 1 1] Crosshair UI
  (bind _returnvalue (UserInterface|CreateWidget "/Game/UI/WB_Crosshair.WB_Crosshair_C"))
  (UserInterface|Viewport|AddtoViewport _returnvalue 0)
  ;[1 1 1] create widget
  (bind _returnvalue_2 (UserInterface|CreateWidget "/Game/UI/BP_UI.BP_UI_C" (Game|GetPlayerController 0)))
  (bind _output_get (Variables|Default|SetHUD%20Widget _returnvalue_2))
  (UserInterface|Viewport|AddtoViewport _output_get 0)
  ;[1 1 1] Start tutorial
  (Tutorial|StartTutorial))

(event EventTick
  (params (DeltaSeconds :type Float%20%28single-precision%29))
  ;[0 0.7605 0.1746] Event Tick
  (CallFunction|GlowingEffect))

(event Input|ActionEvents|InputActionJump
  (params (Key :type Key%20Structure))
  ;[1 1 1] Action Mappings
  (:Pressed
    (Character|Jump)))

(event Input|AxisEvents|InputAxisTurn
  (params (AxisValue :type Float%20%28single-precision%29))
  ;[1 1 1] Camera
  (Pawn|Input|AddControllerYawInput AxisValue))

(event Input|AxisEvents|InputAxisLookUp
  (params (AxisValue :type Float%20%28single-precision%29))
  ;[1 1 1] Camera
  (Pawn|Input|AddControllerPitchInput AxisValue))

(event Input|AxisEvents|InputAxisMoveForward
  (params (AxisValue :type Float%20%28single-precision%29))
  (bind _capsulecomponent (Variables|Collision|GetCapsuleComponent))
  (bind _speedfactor (Variables|Movement|GetSpeedFactor))
  (bind _returnvalue (Math|Vector|GetForwardVector _capsulecomponent))
  (bind _returnvalue_2 (* _returnvalue _speedfactor))
  ;[1 1 1] Movement
  (Pawn|Input|AddMovementInput _returnvalue_2 AxisValue false)
  (Movement|UpdateCurrentSpeedForward _returnvalue_2 AxisValue))

(event Input|AxisEvents|InputAxisMoveRight
  (params (AxisValue :type Float%20%28single-precision%29))
  (bind _capsulecomponent (Variables|Collision|GetCapsuleComponent))
  (bind _speedfactor (Variables|Movement|GetSpeedFactor))
  (bind _returnvalue (Math|Vector|GetRightVector _capsulecomponent))
  (bind _returnvalue_2 (* _returnvalue _speedfactor))
  ;[1 1 1] Movement
  (Pawn|Input|AddMovementInput _returnvalue_2 AxisValue false)
  (Movement|UpdateCurrentSpeedRight _returnvalue_2 AxisValue))

(event Input|KeyboardEvents|DebugKey1
  (params (Key :type Key%20Structure) (ActionValue :type Input%20Action%20Value%20Structure))
  (:Pressed
    (Default|DecreaseHealth (Variables|Default|GetBPC_PlayerStats) 1e+01)))

(event Input|KeyboardEvents|W
  (params (Key :type Key%20Structure))
  (:Pressed
    (bind _stepcomplete (Tutorial|CheckInput "NewEnumerator0"))
    (if _stepcomplete
      (Tutorial|AdvanceStep "NewEnumerator1")
      (Development|PrintString "PressS"))))

(event Input|KeyboardEvents|E
  (params (Key :type Key%20Structure))
  (:Pressed
    (bind _stepcomplete (Tutorial|CheckInput "NewEnumerator5"))
    (if _stepcomplete
      (Tutorial|EndTutorial)
      (Development|PrintString "Finished"))))

(event Input|KeyboardEvents|S
  (params (Key :type Key%20Structure))
  (:Pressed
    (bind _stepcomplete (Tutorial|CheckInput "NewEnumerator1"))
    (if _stepcomplete
      (Tutorial|AdvanceStep "NewEnumerator2")
      (Development|PrintString "PressA"))))

(event Input|KeyboardEvents|A
  (params (Key :type Key%20Structure))
  (:Pressed
    (bind _stepcomplete (Tutorial|CheckInput "NewEnumerator2"))
    (if _stepcomplete
      (Tutorial|AdvanceStep "NewEnumerator3")
      (Development|PrintString "PressD"))))

(event Input|KeyboardEvents|D
  (params (Key :type Key%20Structure))
  (:Pressed
    (bind _stepcomplete (Tutorial|CheckInput "NewEnumerator3"))
    (if _stepcomplete
      (Tutorial|AdvanceStep "NewEnumerator4")
      (Development|PrintString "PressSpace"))))

(event Input|KeyboardEvents|SpaceBar
  (params (Key :type Key%20Structure))
  (:Pressed
    (bind _stepcomplete (Tutorial|CheckInput "NewEnumerator4"))
    (if _stepcomplete
      (Tutorial|AdvanceStep "NewEnumerator5")
      (Development|PrintString "PressE"))))

(event Input|MouseEvents|LeftMouseButton
  (params (Key :type Key%20Structure))
  ;[1 1 1] Punch logic
  (:Pressed
    (Animation|PlayAnimMontage "/Game/Animations/PunchingAnimation_Montage.PunchingAnimation_Montage" 1.0 "None")
    (Utilities|FlowControl|Delay 0.6)
    (Audio|PlaySound2D "/Game/Audio/punchSound.punchSound" 1.0 1.0 0.0 0 0)))

(event Input|KeyboardEvents|T
  (params (Key :type Key%20Structure))
  (bind _camera (Variables|Default|GetCamera))
  ;[1 1 1] just for fun, delete later haha
  (:Pressed
    (Game|SpawnActorfromClass "/Game/Blueprints/PickingUpSystem/BP_item.BP_item_C" (Math|Transform|MakeTransform (+ (Transformation|GetWorldLocation _camera) (* (Math|Vector|Normalize (Math|Vector|GetForwardVector _camera)) (Variables|PickUpSystem|GetPlaceDistance))) "0, 0, 0" "1.000000,1.000000,1.000000") "Undefined" "MultiplyWithRoot" 0 (Variables|/Script/Engine.StaticMeshComponent|GetStaticMesh (Variables|Default|GetEquipedItem)) "NewEnumerator0" 0)
    (Audio|PlaySound2D "/Game/Audio/place_item.place_item" 1.0 1.0 0.0 0 0)))

(event Input|KeyboardEvents|E
  (params (Key :type Key%20Structure))
  ;[1 1 1] Open/Close Turniket Character Logic
  (:Pressed
    (CallFunction|PointHand)
    (Utilities|FlowControl|Delay 0.6)
    (bind (_outhit _returnvalue) (CallFunction|GetRayTracedItem (Variables|Turniket|GetOpenTurniketDistance)))
    (if _returnvalue
      (if (Actor|ActorHasTag (.HitActor (Collision|BreakHitResult _outhit)) "isicTerminal")
        (if (CallFunction|HasIsicFunc)
          (bind _outactors (Actor|GetAllActorswithTag "Turniket"))
          (for _array_element _outactors
            (bind _asbp_pillar_logic (Utilities|Casting|CastToBP_pillar_logic _array_element))
            ;;[1 0.3564 0.3564] basically, the door opens, waits 3 sec and closes
            (Default|OpenDoor _asbp_pillar_logic)
            (Utilities|FlowControl|Delay 3.0)
            (Default|OpenDoor _asbp_pillar_logic))
          (else
            (Audio|PlaySound2D "/Game/Audio/recordered18dec/accessDenied2.accessDenied2" 1.0 1.0 0.0 0 0)))))))

(event Input|KeyboardEvents|Q
  (params (Key :type Key%20Structure))
  ;[1 1 1] Place Item / Pick Up Item Logic
  (:Pressed
    (if (Utilities|Enum|Equal(Enum) (Variables|Inventar|GetHeldItemType) "NewEnumerator0")
      (CallFunction|PickUpItem)
      (else
        (CallFunction|PlaceItem)))))

(fn ConstructionScript)

(fn UpdateCurrentSpeedForward
  (params (Movement%20Input :type Vector) (Speed :type Float%20%28double-precision%29))
  (if (!= (Math|Vector|VectorLength Movement%20Input) 0.0)
    (Variables|Movement|SetCurrentSpeedForward Speed)
    (else
      (Variables|Movement|SetCurrentSpeedForward 0.0))))

(fn UpdateCurrentSpeedRight
  (params (Movement%20input :type Vector) (Speed :type Float%20%28double-precision%29))
  (if (!= (Math|Vector|VectorLength Movement%20input) 0.0)
    (Variables|Movement|SetCurrentSpeedRight Speed)
    (else
      (Variables|Movement|SetCurrentSpeedRight 0.0))))

(fn GetCurrentSpeedForward
  (return (Variables|Movement|GetCurrentSpeedForward)))

(fn GetCurrentSpeedRight
  (return (Variables|Movement|GetCurrentSpeedRight)))

(fn GetRayTracedItem
  (params (RayDistance :type Float%20%28double-precision%29))
  (bind _camera (Variables|Default|GetCamera))
  (bind _returnvalue (Transformation|GetWorldLocation _camera))
  (bind (_outhit _returnvalue_2) (Collision|LineTraceByChannel _returnvalue (+ _returnvalue (* (Math|Vector|GetForwardVector _camera) RayDistance)) "TraceTypeQuery1" false 0 "None" true "(R=1.000000,G=0.000000,B=0.000000,A=1.000000)" "(R=0.000000,G=1.000000,B=0.000000,A=1.000000)" 1.0))
  (return _outhit _returnvalue_2))

(fn GetIsPointingHand
  (return (Variables|Turniket|GetIsPointingHand)))

(fn HasIsicFunc
  (return (Utilities|Enum|Equal(Enum) (Variables|Inventar|GetHeldItemType) "NewEnumerator1")))

(fn TakeLocationforPlace
  (params (Location :type Vector) (EndTraceLocation :type Vector))
  (if (Utilities|Operators|EqualEqual :A Location)
    (Variables|PickUpSystem|SetReturnLocationForPlace EndTraceLocation)
    (else
      (Variables|PickUpSystem|SetReturnLocationForPlace Location)))
  (return (Variables|PickUpSystem|GetReturnLocationForPlace)))

(fn Die
  (bind _camera (Variables|Default|GetCamera))
  (bind _returnvalue (Transformation|GetWorldLocation _camera))
  (SaveGame|DeleteGameinSlot "SavedState")
  (Components|Animation|PlayAnimation (Variables|Character|GetMesh) "/Game/Animations/Dying.Dying" false)
  (Transformation|SetWorldLocation _camera (Math|Vector|MakeVector (- (.x _returnvalue) 1.5e+02) (.y _returnvalue) (- (.z _returnvalue) 5e+01)) false false))

(fn AdvanceStep
  (params (Next%20Step :type TutorialStep%20Enum :default "NewEnumerator0"))
  (Variables|Tutorial|SetTutorialStep Next%20Step))

(fn CheckInput
  (params (Input :type TutorialStep%20Enum :default "NewEnumerator0"))
  (return (Utilities|Enum|Equal(Enum) Input (Variables|Tutorial|GetTutorialStep))))

(fn StartTutorial
  (Tutorial|AdvanceStep "NewEnumerator0")
  (Variables|Tutorial|SetIsTutorial true))

(fn EndTutorial
  (Tutorial|AdvanceStep "NewEnumerator6")
  (Variables|Tutorial|SetIsTutorial false))

(fn ProcessForwardVectorTutorial
  (params (AxisValue :type Float%20%28double-precision%29))
  (bind _speedfactor (Variables|Movement|GetSpeedFactor))
  (bind _capsulecomponent (Variables|Collision|GetCapsuleComponent))
  (bind _returnvalue (Math|Vector|GetForwardVector _capsulecomponent))
  (bind _returnvalue_2 (* _returnvalue _speedfactor))
  (if (!= AxisValue 0.0)
    (if (> AxisValue 0.0)
      (bind _stepcomplete (Tutorial|CheckInput "NewEnumerator0"))
      (if _stepcomplete
        (Tutorial|AdvanceStep "NewEnumerator1")
        (Development|PrintString "PressS")
        (Pawn|Input|AddMovementInput _returnvalue_2 AxisValue false :!label _label)
        (Movement|UpdateCurrentSpeedForward _returnvalue_2 AxisValue))
      (else
        (bind _stepcomplete_2 (Tutorial|CheckInput "NewEnumerator1"))
        (if _stepcomplete_2
          (Tutorial|AdvanceStep "NewEnumerator2")
          (Development|PrintString "PressA")
          (goto _label))))
    (else
      (Movement|UpdateCurrentSpeedForward "0, 0, 0" 0.0))))

(fn ProcessRightVectorTutorial
  (params (AxisValue :type Float%20%28double-precision%29))
  (bind _capsulecomponent (Variables|Collision|GetCapsuleComponent))
  (bind _speedfactor (Variables|Movement|GetSpeedFactor))
  (bind _returnvalue (Math|Vector|GetRightVector _capsulecomponent))
  (bind _returnvalue_2 (* _returnvalue _speedfactor))
  (if (!= AxisValue 0.0)
    (if (> AxisValue 0.0)
      (bind _stepcomplete (Tutorial|CheckInput "NewEnumerator3"))
      (if _stepcomplete
        (Tutorial|AdvanceStep "NewEnumerator4")
        (Development|PrintString "PressSpace")
        (Pawn|Input|AddMovementInput _returnvalue_2 AxisValue false :!label _label)
        (Movement|UpdateCurrentSpeedRight _returnvalue_2 AxisValue))
      (else
        (bind _stepcomplete_2 (Tutorial|CheckInput "NewEnumerator2"))
        (if _stepcomplete_2
          (Tutorial|AdvanceStep "NewEnumerator3")
          (Development|PrintString "PressD")
          (goto _label))))
    (else
      (Movement|UpdateCurrentSpeedRight "0, 0, 0" 0.0))))
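; BP_Door is a hinged door that alternately opens and closes each time its OpenDoor event is called.
; A FlipFlop plays OpenDoorTimeline from the start or reverses it, with a different creak sound for each direction.
; The timeline's float lerps the Door's yaw to 90 degrees and the Klucka handle's pitch to 180.
; When the timeline finishes, a bang sound plays in 2D, like the creaks.
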(event Custom|Open%20Door
  (Utilities|FlowControl|FlipFlop
    (:A
      (Audio|PlaySound2D "/Game/Audio/fromInternet/creaky_door.creaky_door" 1.0 1.0 0.0 0 0)
      (bind _doorfloat (Timeline|OpenDoorTimeline PlayFromStart)
        (:Update
          (Transformation|SetRelativeRotation (Variables|Default|GetDoor) (Math|Rotator|MakeRotator 0.0 0.0 (Math|Float|Lerp 0.0 9e+01 _doorfloat)) false false)
          (Transformation|SetRelativeRotation (Variables|Default|GetKlucka) (Math|Rotator|MakeRotator 0.0 (Math|Float|Lerp 0.0 1.8e+02 _doorfloat) 0.0) false false))
        (:Finished
          (Audio|PlaySound2D "/Game/Audio/recordered18dec/booomTrashbin.booomTrashbin" 1.0 1.0 0.0 0 0))))
    (:B
      (Audio|PlaySound2D "/Game/Audio/fromInternet/creaky_door2.creaky_door2" 1.0 1.0 0.0 0 0)
      (Timeline|OpenDoorTimeline Reverse))))

(fn ConstructionScript)
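; Enemy monster AI that chases the player on sight and deals bite damage.
; PawnSensing triggers an AIMoveTo toward the player, whose immediate Then output, not move success, runs the CanAttack-gated damage.
; Capsule overlaps jump straight into that damage step without checking the gate or overlapping actor.
; Damage goes through the player's stats component, calling death logic when it reports true; Tick halts movement until the player is seen.
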(event OnSeePawn(PawnSensing)
  (params (Pawn :type Pawn%20Object%20Reference))
  (Variables|Default|SetisSeeingPlayer true)
  (CallFunction|FollowPlayer))

(event OnComponentBeginOverlap(CapsuleComponent)
  (params (OverlappedComponent :type Primitive%20Component%20Object%20Reference) (OtherActor :type Actor%20Object%20Reference) (OtherComp :type Primitive%20Component%20Object%20Reference) (OtherBodyIndex :type Integer) (bFromSweep :type Boolean) (SweepResult :type Hit%20Result%20Structure%20%28by%20ref%29))
  (bind _asbp_fps_character (Utilities|Casting|CastToBP_FPS_Character (Game|Player|GetPlayerPawn 0)))
  (bind _is_player_dead (Default|DecreaseHealth (Variables|/Game/Blueprints/Character/BP_FPS_Character.BP_FPS_Character_C|GetBPC_PlayerStats _asbp_fps_character) 1.0))
  (Audio|PlaySoundatLocation "/Game/Audio/fromInternet/monster_biting.monster_biting" (Transformation|GetActorLocation) "0, 0, 0" 0.3 1.0 0.0 0 0 0 0)
  (if _is_player_dead
    (Default|DiyingLogic _asbp_fps_character)
    (else
      (Variables|Default|SetcanAttack true))))

(event Custom|FollowPlayer
  (Variables|Default|SetcanAttack true)
  (if (Variables|Default|GetisSeeingPlayer)
    (AI|AIMoveTo self "0, 0, 0" (Game|GetPlayerCharacter 0) 0.0 false
      (:then
        (if (Variables|Default|GetcanAttack)
          (Variables|Default|SetcanAttack false)
          (bind _asbp_fps_character (Utilities|Casting|CastToBP_FPS_Character (Game|Player|GetPlayerPawn 0)))
          (bind _is_player_dead (Default|DecreaseHealth (Variables|/Game/Blueprints/Character/BP_FPS_Character.BP_FPS_Character_C|GetBPC_PlayerStats _asbp_fps_character) 1.0))
          (Audio|PlaySoundatLocation "/Game/Audio/fromInternet/monster_biting.monster_biting" (Transformation|GetActorLocation) "0, 0, 0" 0.3 1.0 0.0 0 0 0 0)
          (if _is_player_dead
            (Default|DiyingLogic _asbp_fps_character)
            (else
              (Variables|Default|SetcanAttack true))))))
    (else
      (Variables|Default|SetisSeeingPlayer false))))

(event Custom|OnActorBeginOverlap_Event
  (params (OverlappedActor :type Actor%20Object%20Reference) (OtherActor :type Actor%20Object%20Reference))
  (bind _asbp_fps_character (Utilities|Casting|CastToBP_FPS_Character (Game|Player|GetPlayerPawn 0)))
  (bind _is_player_dead (Default|DecreaseHealth (Variables|/Game/Blueprints/Character/BP_FPS_Character.BP_FPS_Character_C|GetBPC_PlayerStats _asbp_fps_character) 1.0))
  (Audio|PlaySoundatLocation "/Game/Audio/fromInternet/monster_biting.monster_biting" (Transformation|GetActorLocation) "0, 0, 0" 0.3 1.0 0.0 0 0 0 0)
  (if _is_player_dead
    (Default|DiyingLogic _asbp_fps_character)
    (else
      (Variables|Default|SetcanAttack true))))

(event EventBeginPlay
  (Audio|PlaySoundatLocation "/Game/Audio/fromInternet/monster_spawn.monster_spawn" (Transformation|GetActorLocation) "0, 0, 0" 0.2 1.0 0.0 "/Game/Audio/SoundAssets/NatureSoundAttenuation.NatureSoundAttenuation" 0 0 0))

(event Collision|EventActorBeginOverlap
  (params (OtherActor :type Actor%20Object%20Reference)))

(event EventTick
  (params (DeltaSeconds :type Float%20%28single-precision%29))
  (if (not (Variables|Default|GetisSeeingPlayer))
    (Components|Movement|StopMovementImmediately (Variables|Character|GetCharacterMovement))))

(fn ConstructionScript)
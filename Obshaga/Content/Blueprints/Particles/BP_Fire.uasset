(event Custom|Activate%20Fire
  (Components|Activation|Activate (Variables|Default|GetFire) false)
  (Components|Activation|Activate (Variables|Default|GetSound) false)
  (Variables|Default|SetFire%20active true))

(event Custom|Start%20Timer
  (Utilities|Time|SetTimerbyFunctionName 0 "Loose" 3e+01))

(event EventTick
  (params (DeltaSeconds :type Float%20%28single-precision%29))
  (if (Variables|Default|GetFire%20active)
    (for _array_element (Collision|GetOverlappingActors "/Game/Blueprints/PickingUpSystem/BP_item.BP_item_C" :!class /Script/Engine.Actor)
      (bind _asbp_item (Utilities|Casting|CastToBP_item _array_element))
      (if (Utilities|Enum|Equal(Enum) (Variables|/Game/Blueprints/PickingUpSystem/BP_item.BP_item_C|GetItemType _asbp_item) "NewEnumerator5")
        (Components|Activation|Deactivate (Variables|Default|GetFire))
        (Components|Activation|Deactivate (Variables|Default|GetSound))
        (bind _asbp_fps_character (Utilities|Casting|CastToBP_FPS_Character (Game|GetPlayerCharacter 0)))
        (Utilities|FlowControl|DoOnce false
          (:Completed
            (Default|MakeInfoNotification _asbp_fps_character "Thank you! You saved the dorms")
            (Utilities|Time|ClearTimerbyFunctionName 0 "Loose")))))))

(fn ConstructionScript)

(fn Loose
  (bind _asbp_fps_character (Utilities|Casting|CastToBP_FPS_Character (Game|GetPlayerCharacter 0)))
  (Default|MakeInfoNotification _asbp_fps_character "You lost, fire destroyed dorms")
  (Default|DiyingLogic _asbp_fps_character))
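; Power-up actor for the pickup system, with a configurable mesh and a floating text label.
; The construction script applies the mesh and label text from its variables.
; Any overlap with the Trigger toggles the label's visibility, and Tick rotates the label toward the player camera.
; IsForSell exposes the ForSell flag; no pickup effect is implemented here.
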(event OnComponentBeginOverlap(Trigger)
  (params (OverlappedComponent :type Primitive%20Component%20Object%20Reference) (OtherActor :type Actor%20Object%20Reference) (OtherComp :type Primitive%20Component%20Object%20Reference) (OtherBodyIndex :type Integer) (bFromSweep :type Boolean) (SweepResult :type Hit%20Result%20Structure%20%28by%20ref%29))
  ;[1 1 1] Show/hide text and glow when close enough
  (Rendering|SetVisibility (Variables|Default|GetText) true false))

(event OnComponentEndOverlap(Trigger)
  (params (OverlappedComponent :type Primitive%20Component%20Object%20Reference) (OtherActor :type Actor%20Object%20Reference) (OtherComp :type Primitive%20Component%20Object%20Reference) (OtherBodyIndex :type Integer))
  ;[1 1 1] Show/hide text and glow when close enough
  (Rendering|SetVisibility (Variables|Default|GetText) false false))

(event EventTick
  (params (DeltaSeconds :type Float%20%28single-precision%29))
  ;[1 1 1] Text always face player
  (Transformation|SetWorldRotation (Variables|Default|GetText) (Math|Rotator|FindLookatRotation (Transformation|GetWorldLocation (Variables|Default|GetText)) (Transformation|GetActorLocation (Game|GetPlayerCameraManager 0))) false false))

(fn ConstructionScript
  (Utilities|FlowControl|Sequence
    (:then_0
      (Components|StaticMesh|SetStaticMesh (Variables|Default|GetPowerUpModel) (Variables|Default|GetPowerUpStaticMesh)))
    (:then_1
      (Rendering|Components|TextRender|SetText (Variables|Default|GetText) (Variables|Default|GetPowerUpUpperText)))))

(fn IsforSell
  (return (Variables|Default|GetforSell)))